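; Wolf enemy that roams randomly, chases the first-person player and bites at close range.
; PawnSensing sends it to heard player positions at any time, while Tick enables sight only at night via the GameInstance's Day flag.
; Delay loops drive wandering, night pursuit and repeated damage while the player overlaps its Box.
; Animations play directly on the mesh; IsHeard is set but never read here.
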(event OnComponentBeginOverlap(Box)
  (params (OverlappedComponent :type Primitive%20Component%20Object%20Reference) (OtherActor :type Actor%20Object%20Reference) (OtherComp :type Primitive%20Component%20Object%20Reference) (OtherBodyIndex :type Integer) (bFromSweep :type Boolean) (SweepResult :type Hit%20Result%20Structure%20%28by%20ref%29))
  ;[1 1 1] Bite and damage mechanic
  (bind _asbp_first_person_character (Utilities|Casting|CastToBP_FirstPersonCharacter OtherActor))
  (Variables|/Game/FirstPerson/Blueprints/BP_FirstPersonCharacter.BP_FirstPersonCharacter_C|SetDamageAmmount _asbp_first_person_character 10)
  (Variables|Default|SetisInBox? true)
  (if (Variables|Default|GetisInBox?) :!label _label
    (Components|Animation|PlayAnimation (Variables|Character|GetMesh) "/Game/AnimalVarietyPack/Wolf/Animations/Woolfbitesoundeffect.Woolfbitesoundeffect" false)
    (Utilities|FlowControl|Delay 0.4)
    (Default|Damage _asbp_first_person_character)
    (Utilities|FlowControl|Delay 0.4)
    (goto _label)))

(event OnComponentEndOverlap(Box)
  (params (OverlappedComponent :type Primitive%20Component%20Object%20Reference) (OtherActor :type Actor%20Object%20Reference) (OtherComp :type Primitive%20Component%20Object%20Reference) (OtherBodyIndex :type Integer))
  ;[1 1 1] Bite and damage mechanic
  (Utilities|Casting|CastToBP_FirstPersonCharacter OtherActor)
  (Variables|Default|SetisInBox? false))

(event OnSeePawn(PawnSensing)
  (params (Pawn :type Pawn%20Object%20Reference))
  (if (not (Variables|/Game/BP_GameInstance.BP_GameInstance_C|GetDay? (stale EventTick _asbp_game_instance))) :!label _label
    (bind _asbp_first_person_character (Utilities|Casting|CastToBP_FirstPersonCharacter Pawn))
    (Variables|Default|SetisHeard? true)
    (Components|Animation|PlayAnimation (Variables|Character|GetMesh) "/Game/AnimalVarietyPack/Wolf/Animations/AM_WolfRun.AM_WolfRun" true)
    (AI|AIMoveTo self (Transformation|GetActorLocation _asbp_first_person_character) 0 5.0 false
      (:OnSuccess
        (Variables|Default|SetisHeard? false)
        (Components|Animation|PlayAnimation (Variables|Character|GetMesh) "/Game/AnimalVarietyPack/Wolf/Animations/ANIM_Wolf_IdleLookAround.ANIM_Wolf_IdleLookAround" true)
        (Utilities|FlowControl|Delay 2.0)
        (goto _label)))))

(event OnHearNoise(PawnSensing)
  (params (Instigator :type Pawn%20Object%20Reference) (Location :type Vector%20%28by%20ref%29 :default "0, 0, 0") (Volume :type Float%20%28single-precision%29))
  ;[1 1 1] Hear Mechanic
  (bind _asbp_first_person_character (Utilities|Casting|CastToBP_FirstPersonCharacter Instigator))
  (Variables|Default|SetisHeard? true)
  (bind _output_get (Variables|Default|Setlocation (Transformation|GetActorLocation _asbp_first_person_character)))
  (Components|Animation|PlayAnimation (Variables|Character|GetMesh) "/Game/AnimalVarietyPack/Wolf/Animations/ANIM_Wolf_Run.ANIM_Wolf_Run" true)
  (AI|AIMoveTo self _output_get 0 5.0 false
    (:OnSuccess
      (Variables|Default|SetisHeard? false)
      (Components|Animation|PlayAnimation (Variables|Character|GetMesh) "/Game/AnimalVarietyPack/Wolf/Animations/ANIM_Wolf_IdleLookAround.ANIM_Wolf_IdleLookAround" true)
      (Utilities|FlowControl|Delay 2.0)
      (CallFunction|WalkRandom))))

(event Custom|WalkRandom
  ;[1 1 1] Walk Random
  (Utilities|FlowControl|Sequence
    (:then_0
      (if true :!label _label
        (Components|Animation|PlayAnimation (Variables|Character|GetMesh) "/Game/AnimalVarietyPack/Wolf/Animations/ANIM_Wolf_Run.ANIM_Wolf_Run" true)
        (AI|AIMoveTo self (.RandomLocation (AI|Navigation|GetRandomReachablePointinRadius (Transformation|GetActorLocation) 1.5e+03 0 0)) 0 5.0 false
          (:OnSuccess
            (Components|Animation|PlayAnimation (Variables|Character|GetMesh) "/Game/AnimalVarietyPack/Wolf/Animations/ANIM_Wolf_IdleBreathe.ANIM_Wolf_IdleBreathe" true)
            (Utilities|FlowControl|Delay 2.0)
            (goto _label)))))))

(event EventTick
  (params (DeltaSeconds :type Float%20%28single-precision%29))
  (bind _pawnsensing (Variables|Default|GetPawnSensing))
  (bind _asbp_game_instance (Utilities|Casting|CastToBP_GameInstance (Game|GetGameInstance)))
  (if (Variables|/Game/BP_GameInstance.BP_GameInstance_C|GetDay? _asbp_game_instance)
    (Variables|/Script/AIModule.PawnSensingComponent|SetbSeePawns _pawnsensing false)
    (else
      (Variables|/Script/AIModule.PawnSensingComponent|SetbSeePawns _pawnsensing true))))

(event EventBeginPlay
  ;[1 1 1] Walk Random
  (CallFunction|WalkRandom))

(fn ConstructionScript)