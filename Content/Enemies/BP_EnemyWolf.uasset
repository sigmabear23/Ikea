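; Enemy wolf that wakes when it hears a noise, then pursues the player and can hurt or kill them.
; Hearing swaps the visible mesh, plays a one-time get-up animation, then after a short delay issues an AI move toward the player with a very large acceptance radius.
; Box overlap calls Damage on the first-person character, while a separate overlap-style custom event, with no binding shown here, calls Death.
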(event OnHearNoise(PawnSensing)
  (params (Instigator :type Pawn%20Object%20Reference) (Location :type Vector%20%28by%20ref%29 :default "0, 0, 0") (Volume :type Float%20%28single-precision%29))
  (Rendering|SetVisibility (Variables|Default|GetMesh%20%28CharacterMesh0%29) true false)
  (if (Variables|Default|GetHeard?)
    _
    (else
      (Variables|Default|SetHeard? true)
      (Components|Animation|PlayAnimation (Variables|Default|GetMesh%20%28CharacterMesh0%29) "/Game/AnimalVarietyPack/Wolf/Animations/ANIM_Wolf_RestToGoBackUp.ANIM_Wolf_RestToGoBackUp" false)))
  (Rendering|SetVisibility (Variables|Default|GetCharacterMesh1) false false)
  (Variables|Default|SetisSeeingPlayer? true)
  (Utilities|FlowControl|Delay 1.4)
  (CallFunction|FollowPlayer))

(event OnComponentBeginOverlap(Box)
  (params (OverlappedComponent :type Primitive%20Component%20Object%20Reference) (OtherActor :type Actor%20Object%20Reference) (OtherComp :type Primitive%20Component%20Object%20Reference) (OtherBodyIndex :type Integer) (bFromSweep :type Boolean) (SweepResult :type Hit%20Result%20Structure%20%28by%20ref%29))
  (bind _asbp_first_person_character (Utilities|Casting|CastToBP_FirstPersonCharacter OtherActor))
  (Default|Damage _asbp_first_person_character))

(event Custom|CustomEvent
  (params (OverlappedComponent :type Primitive%20Component%20Object%20Reference) (OtherActor :type Actor%20Object%20Reference) (OtherComp :type Primitive%20Component%20Object%20Reference) (OtherBodyIndex :type Integer) (bFromSweep :type Boolean) (SweepResult :type Hit%20Result%20Structure%20%28by%20ref%29))
  (Components|Animation|PlayAnimation (Variables|Default|GetMesh%20%28CharacterMesh0%29) 0 false)
  (bind _asbp_first_person_character (Utilities|Casting|CastToBP_FirstPersonCharacter OtherActor))
  (Default|Death _asbp_first_person_character))

(event Custom|FollowPlayer
  (if (Variables|Default|GetisSeeingPlayer?)
    (AI|AIMoveTo self "0, 0, 0" (Game|GetPlayerCharacter 0) 9e+03 false)))

(fn ConstructionScript)