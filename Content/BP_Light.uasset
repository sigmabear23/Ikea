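; BP_Light is a flickering light actor that briefly cuts out at random intervals.
; BeginPlay runs an endless loop: after a random delay of a few seconds, it hides the SpotLight and swaps the LightOn component for LightOff.
; After a random fraction of a second it restores both, then repeats through a wire back to the first Delay.
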(event EventBeginPlay
  (Utilities|FlowControl|Delay (Math|Random|RandomFloatinRange 2.0 7.0) :!label _label)
  (Rendering|SetVisibility (Variables|Default|GetSpotLight) false false)
  (Rendering|SetVisibility (Variables|Default|GetLightOn) false false)
  (Rendering|SetVisibility (Variables|Default|GetLightOff) true false)
  (Utilities|FlowControl|Delay (Math|Random|RandomFloatinRange 0.1 0.3))
  (Rendering|SetVisibility (Variables|Default|GetSpotLight) true false)
  (Rendering|SetVisibility (Variables|Default|GetLightOn) true false)
  (Rendering|SetVisibility (Variables|Default|GetLightOff) false false)
  (goto _label))

(fn ConstructionScript)